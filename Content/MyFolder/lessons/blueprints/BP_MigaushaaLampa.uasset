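; Blinking lamp actor that flashes its SpotLight on and off continuously.
; Tick feeds a 0.2-second Delay, which throttles a FlipFlop that alternates IsEnabled and drives the light's visibility.
; The construction script applies IsEnabled to the SpotLight to set its initial visibility.
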(event EventBeginPlay)

(event Collision|EventActorBeginOverlap
  (params (OtherActor :type Actor%20Object%20Reference)))

(event EventTick
  (params (DeltaSeconds :type Float%20%28single-precision%29))
  (Utilities|FlowControl|Delay 0.2)
  (Utilities|FlowControl|FlipFlop
    (:A
      (Variables|Default|SetIsEnabled true))
    (:B
      (Variables|Default|SetIsEnabled false)))
  (Rendering|SetVisibility (Variables|Default|GetSpotLight) (Variables|Default|GetIsEnabled) false))

(fn ConstructionScript
  (Rendering|SetVisibility (Variables|Default|GetSpotLight) (Variables|Default|GetIsEnabled) false))